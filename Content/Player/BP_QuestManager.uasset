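; BP_QuestManager checks daily quest completion based on the action animation of the guardian player's current prisoner.
; DaysQuestController casts the first player controller to BP_GuardianPlayer and maps each of seven days to a required prisoner action, always using quest ID zero.
; ControllBool compares that action with the prisoner's ActionAnimation and passes the result to SetQuestBool, with both branches making the same call.
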(event `DaysQuestController`
  (params (Day :type Integer))
  (bind _asbp_guardian_player (cast `/Game/Player/Input/BP_GuardianPlayer` (`GameplayStatics.GetPlayerController` 0)))
  (switch `int` Day
    (:`0`
      (`self.ControllBool` _asbp_guardian_player "Mirroring"))
    (:`1`
      (`self.ControllBool` _asbp_guardian_player "ThrowCoin"))
    (:`2`
      (`self.ControllBool` _asbp_guardian_player "Give"))
    (:`3`
      (`self.ControllBool` _asbp_guardian_player "Eat"))
    (:`4`
      (`self.ControllBool` _asbp_guardian_player "LazeAround"))
    (:`5`
      (`self.ControllBool` _asbp_guardian_player "Read"))
    (:`6`
      (`self.ControllBool` _asbp_guardian_player "Fight"))))

(fn `ControllBool`
  (params (Controller :type "/Game/Player/Input/BP_GuardianPlayer Object Reference") (Action :type "EActionAnimation Enum" :default "BaseLocomotion") (Quest :type Integer))
  (bind _returnvalue (`|EnumEquality` (`PrisonerCharacter.ActionAnimation` (`PrisonerCharacterController.Prisoner` (`GuardianPlayerController.CurrentController` Controller))) Action))
  (if _returnvalue
    (`self.SetQuestBool` Quest _returnvalue)
    (else
      (`self.SetQuestBool` Quest _returnvalue))))

(fn `UserConstructionScript`)