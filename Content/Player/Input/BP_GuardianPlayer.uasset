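; Guardian player controller that links prisoner setup, camera switching and the BP_GuardianHUD cached at BeginPlay.
; PrisonerSetup fills each PrisonersController entry's stats from the DT_PrisonerStats row at the same index.
; Camera changes optionally play a timeline that lerps the current cine camera's rotation, then call ChangeCamera and update the HUD menu.
; Selection and deselection events show or hide the current prisoner through the HUD.
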(event `self.ReceiveBeginPlay`
  (bind _asbp_guardian_hud (cast `/Game/UserInterface/BP_GuardianHUD` (`self.GetHUD`)))
  (set `self.Hud` _asbp_guardian_hud))

(event `self.StartPrisonerParameter`
  (`self.PrisonerSetup`))

(event `self.CameraChangeRotation`
  (bind _cinecameracomponent (`PlayerCamera.CineCameraComponent` (`self.CameraCurrentRot`)))
  (if (`self.WaitToCameraRot`)
    (bind (_direction _rotatiolerp) (`Timeline|RotateCamera` :!via `PlayFromStart`)
      (:`Update`
        (`SceneComponent.K2_SetRelativeRotation` _cinecameracomponent (`KismetMathLibrary.RLerp` (`SceneComponent.RelativeRotation` _cinecameracomponent) (`self.CameraRot`) _rotatiolerp) false false))
      (:`Finished`
        (`self.ChangeCamera` :!label _label)
        (`/Game/UserInterface/BP_GuardianHUD.UISetMailMenu` (`self.Hud`) (`self.WaitToCameraRot`))))
    (else
      (goto _label))))

(event `self.DeselectPrisonerVisibility`
  (`/Game/UserInterface/BP_GuardianHUD.VisualizePrisoner` (`self.Hud`) "Hidden" (`self.CurrentID`)))

(event `self.SelectedPrisonerVisibility`
  (`/Game/UserInterface/BP_GuardianHUD.VisualizePrisoner` (`self.Hud`) "Visible" (`self.CurrentID`)))

(fn `PrisonerSetup`
  (for (_ _array_index) (`self.PrisonersController`)
    (bind _outrownames (`DataTableFunctionLibrary.GetDataTableRowNames` "/Game/Datatables/DT_PrisonerStats.DT_PrisonerStats"))
    (bind _returnvalue (`|GetDataTableRow` "/Game/Datatables/DT_PrisonerStats.DT_PrisonerStats" (`|GetArrayItem` _outrownames _array_index))
      (:`then`
        (set `PrisonerCharacterController.Stats` (break `DataPrisoner` _returnvalue) (`|GetArrayItem` (`self.PrisonersController`) _array_index))))))

(fn `UserConstructionScript`)