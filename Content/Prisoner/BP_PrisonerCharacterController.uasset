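; AI controller for the prisoner character that starts its behavior tree on possess and seeds the wander point and wait time.
; Each tick it feeds the blackboard the player-control flag, the guardian player's cached mouse destination and the prisoner's current action.
; A real-time timeout ends non-death actions that run too long, dropping player control and resetting the random point to the prisoner's location.
; TreeSettings resets the action state to base locomotion.
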(event `self.ReceiveBeginPlay`)

(event `self.ReceiveTick`
  (params (DeltaSeconds :type "Float (single-precision)"))
  (bind _returnvalue (`GameplayStatics.GetRealTimeSeconds`))
  (bind _blackboard (`self.Blackboard`))
  (bind _prisoner (`self.Prisoner`))
  (bind _blackboard_2 (`self.Blackboard`))
  (bind _actionanimation (`PrisonerCharacter.ActionAnimation` _prisoner))
  (if (`self.BTActive`)
    (if (`self.IsPlayerControlled`)
      (set `self.Controlled` 1)
      (else
        (set `self.Controlled` 0)))
    (`BlackboardComponent.SetValueAsInt` _blackboard "IsPlayerControlled" (`self.Controlled`))
    (bind _asbp_guardian_player (cast `/Game/Player/Input/BP_GuardianPlayer` (`GameplayStatics.GetPlayerController` 0)))
    (`BlackboardComponent.SetValueAsVector` _blackboard "MousePosition" (`GuardianPlayerController.CachedDestination` _asbp_guardian_player))
    (`BlackboardComponent.SetValueAsEnum` (`self.Blackboard`) "Action" _actionanimation)
    (if (and (`|EnumInequality` _actionanimation "Dead") (`PrisonerCharacter.IsInAction` _prisoner))
      (if (> (`self.TimerAction`) (`self.TimerToWaitACtion`))
        (set `self.IsPlayerControlled` false)
        (set `PrisonerCharacter.IsInAction` false (`self.Prisoner`))
        (`BlackboardComponent.SetValueAsInt` _blackboard_2 "ActionUsed" 0)
        (`BlackboardComponent.SetValueAsVector` _blackboard_2 "RandomPoint" (`self.K2_GetActorLocation` (`self.Prisoner`)))
        (else
          (set `self.TimerAction` (`GameplayStatics.GetRealTimeSeconds`))))
      (else
        (set `self.TimerAction` _returnvalue)
        (set `self.TimerToWaitACtion` (+ _returnvalue (`self.AddToWaitAction`)))))))

(event `self.ReceivePossess`
  (params (PossessedPawn :type "Pawn Object Reference"))
  (bind _blackboard (`self.Blackboard`))
  (bind _returnvalue (`self.RunBehaviorTree` (`self.BT`)))
  (set `self.BTActive` _returnvalue)
  (`BlackboardComponent.SetValueAsVector` _blackboard "RandomPoint" (`self.K2_GetActorLocation` (`self.Prisoner`)))
  (`BlackboardComponent.SetValueAsFloat` _blackboard "WaitTime" 5.0))

(event `TreeSettings`
  (bind _prisoner (`self.Prisoner`))
  (set `PrisonerCharacter.IsInAction` false _prisoner)
  (set `PrisonerCharacter.ActionAnimation` "BaseLocomotion" _prisoner)
  (`BlackboardComponent.SetValueAsInt` (`self.Blackboard`) "ActionUsed" 0))

(fn `UserConstructionScript`)